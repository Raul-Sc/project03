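; Player robot pawn with a toggleable spotlight, battery pickups, and win and death screens.
; Detector overlaps recharge through a negative DrainBattery call and destroy the battery, or trigger PlayerWin on a Finish actor.
; R asks the game mode to spawn a battery and, if StatusOn is false, toggles status for two seconds.
; Escape flip-flops the pause menu; PlayerDead switches off the light, then, like PlayerWin, shows its widget and pauses.
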(event `Key|R`
  (params (Key :type "Key Structure"))
  (:`Pressed`
    (bind _asb_p_proj_03game_mode_base (cast `/Game/Blueprints/bP_proj_03GameModeBase` (`GameplayStatics.GetGameMode`)))
    (`proj_03GameModeBase.spawnBattery` _asb_p_proj_03game_mode_base)
    (if (not (`self.statusOn`))
      (`self.toggleStatus`)
      (`KismetSystemLibrary.Delay` 2.0)
      (`self.toggleStatus`))))

(event `InputAction|ToggleLight`
  (params (Key :type "Key Structure"))
  (:`Pressed`
    (`SceneComponent.ToggleVisibility` (`self.SpotLight`) false)
    (`self.toggleLight`)))

(event `Key|Escape` :paused true
  (params (Key :type "Key Structure"))
  (:`Pressed`
    (`/Engine/EditorBlueprintResources/StandardMacros.FlipFlop`
      (:`A`
        (bind _returnvalue (`|CreateWidget` "/Game/Blueprints/PauseGame.PauseGame_C"))
        (`UserWidget.AddToViewport` _returnvalue 0)
        (set `PlayerController.bShowMouseCursor` true (`GameplayStatics.GetPlayerController` 0))
        (`GameplayStatics.SetGamePaused` true))
      (:`B`
        (`Widget.RemoveFromParent` _returnvalue)
        (`GameplayStatics.SetGamePaused` false)))))

(event `self.ReceiveBeginPlay`)

(event `self.Detector.OnComponentBeginOverlap`
  (params (OverlappedComponent :type "PrimitiveComponent Object Reference") (OtherActor :type "Actor Object Reference") (OtherComp :type "PrimitiveComponent Object Reference") (OtherBodyIndex :type Integer) (bFromSweep :type Boolean) (SweepResult :type "HitResult Structure (by ref)"))
  (bind _asbp_battery (cast `/Game/BP_Battery` OtherActor)
    (:`then`
      (bind _returnvalue (`Battery.getCharge` _asbp_battery))
      (`self.drainBattery` (* _returnvalue -1.0))
      (`self.K2_DestroyActor` OtherActor))
    (:`CastFailed`
      (cast `/Game/Blueprints/Finish` OtherActor)
      (`self.PlayerWin`))))

(fn `PlayerDead`
  (bind _spotlight (`self.SpotLight`))
  (if (`SceneComponent.IsVisible` _spotlight)
    (`SceneComponent.ToggleVisibility` _spotlight false)
    (`self.toggleLight`))
  (bind _returnvalue (`|CreateWidget` "/Game/Blueprints/GameOver.GameOver_C"))
  (`UserWidget.AddToViewport` _returnvalue 0)
  (set `PlayerController.bShowMouseCursor` true (`GameplayStatics.GetPlayerController` 0))
  (`GameplayStatics.SetGamePaused` true))

(fn `PlayerWin`
  (bind _returnvalue (`|CreateWidget` "/Game/Blueprints/FinishedGame.FinishedGame_C"))
  (`UserWidget.AddToViewport` _returnvalue 0)
  (set `PlayerController.bShowMouseCursor` true (`GameplayStatics.GetPlayerController` 0))
  (`GameplayStatics.SetGamePaused` true))

(fn `UserConstructionScript`)